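; BP_Map is an actor that builds a grid-based level from a text file in its construction script.
; It first lays a floor grid of child actor components below the origin.
; It then reads Files/Map.txt from the project content folder, treating each line as a row and each character as a column.
; Recognised symbols (#, ., B, R, G, Y) each add a child actor at that grid cell, with no runtime logic.
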(fn `UserConstructionScript`
  (for _index (range -5 16)
    (for _index_2 (range -5 16)
      (`AddComponent|NODE_AddChildActorComponent-7` :`RelativeTransform` (`KismetMathLibrary.Conv_VectorToTransform` (`KismetMathLibrary.TransformLocation` (`self.ActorLocation`) (`KismetMathLibrary.MakeVector` (`KismetMathLibrary.Conv_IntToDouble` (* _index 125)) (`KismetMathLibrary.Conv_IntToDouble` (* _index_2 125)) -175.0))))))
  (for (_array_element _array_index) (`FileSDKBPLibrary.ReadLinesFromFile` (`KismetStringLibrary.Concat_StrStr` (`KismetSystemLibrary.GetProjectContentDirectory`) "Files/Map.txt"))
    (set `self.x-Axis` _array_index)
    (for (_array_element_2 _array_index_2) (`KismetStringLibrary.GetCharacterArrayFromString` _array_element)
      (set `self.y-Axis` _array_index_2)
      (set `self.ActorName` _array_element_2)
      (if (`KismetStringLibrary.EqualEqual_StrStr` (`self.ActorName`) "#")
        (`AddComponent|NODE_AddChildActorComponent-0` :`RelativeTransform` (`KismetMathLibrary.Conv_VectorToTransform` (`KismetMathLibrary.TransformLocation` (`self.ActorLocation`) (`KismetMathLibrary.MakeVector` (`KismetMathLibrary.Conv_IntToDouble` (* (`self.x-Axis`) 100)) (`KismetMathLibrary.Conv_IntToDouble` (* (`self.y-Axis`) 100))))))
        (elif (`KismetStringLibrary.EqualEqual_StrStr` (`self.ActorName`) ".")
          (`AddComponent|NODE_AddChildActorComponent-1` :`RelativeTransform` (`KismetMathLibrary.Conv_VectorToTransform` (`KismetMathLibrary.TransformLocation` (`self.ActorLocation`) (`KismetMathLibrary.MakeVector` (`KismetMathLibrary.Conv_IntToDouble` (* (`self.x-Axis`) 100)) (`KismetMathLibrary.Conv_IntToDouble` (* (`self.y-Axis`) 100))))))
          (elif (`KismetStringLibrary.EqualEqual_StrStr` (`self.ActorName`) "B")
            (`AddComponent|NODE_AddChildActorComponent-2` :`RelativeTransform` (`KismetMathLibrary.Conv_VectorToTransform` (`KismetMathLibrary.TransformLocation` (`self.ActorLocation`) (`KismetMathLibrary.MakeVector` (`KismetMathLibrary.Conv_IntToDouble` (* (`self.x-Axis`) 100)) (`KismetMathLibrary.Conv_IntToDouble` (* (`self.y-Axis`) 100))))))
            (elif (`KismetStringLibrary.EqualEqual_StrStr` (`self.ActorName`) "R")
              (`AddComponent|NODE_AddChildActorComponent-4` :`RelativeTransform` (`KismetMathLibrary.Conv_VectorToTransform` (`KismetMathLibrary.TransformLocation` (`self.ActorLocation`) (`KismetMathLibrary.MakeVector` (`KismetMathLibrary.Conv_IntToDouble` (* (`self.x-Axis`) 100)) (`KismetMathLibrary.Conv_IntToDouble` (* (`self.y-Axis`) 100))))))
              (elif (`KismetStringLibrary.EqualEqual_StrStr` (`self.ActorName`) "G")
                (`AddComponent|NODE_AddChildActorComponent-5` :`RelativeTransform` (`KismetMathLibrary.Conv_VectorToTransform` (`KismetMathLibrary.TransformLocation` (`self.ActorLocation`) (`KismetMathLibrary.MakeVector` (`KismetMathLibrary.Conv_IntToDouble` (* (`self.x-Axis`) 100)) (`KismetMathLibrary.Conv_IntToDouble` (* (`self.y-Axis`) 100))))))
                (elif (`KismetStringLibrary.EqualEqual_StrStr` (`self.ActorName`) "Y")
                  (`AddComponent|NODE_AddChildActorComponent-6` :`RelativeTransform` (`KismetMathLibrary.Conv_VectorToTransform` (`KismetMathLibrary.TransformLocation` (`self.ActorLocation`) (`KismetMathLibrary.MakeVector` (`KismetMathLibrary.Conv_IntToDouble` (* (`self.x-Axis`) 100)) (`KismetMathLibrary.Conv_IntToDouble` (* (`self.y-Axis`) 100)))))))))))))))