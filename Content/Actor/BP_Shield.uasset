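; BP_Shield is a pickup actor that grants a shield to a player character that overlaps it.
; On ActorBeginOverlap it tries a chain of casts to the ThirdPersonCharacter, Alex, Alex_Stroumph and Steve_Rouge character Blueprints.
; On a match it sets IsShielded if not already set, then destroys itself even if the character was already shielded; other actors are ignored.
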(event `self.ReceiveActorBeginOverlap`
  (params (OtherActor :type "Actor Object Reference"))
  (bind _asbp_third_person_character (cast `/Game/ThirdPerson/Blueprints/BP_ThirdPersonCharacter` OtherActor)
    (:`then`
      (if (not (`/Game/ThirdPerson/Blueprints/BP_ThirdPersonCharacter.isShielded` _asbp_third_person_character))
        (set `/Game/ThirdPerson/Blueprints/BP_ThirdPersonCharacter.isShielded` true _asbp_third_person_character)))
    (:`CastFailed`
      (bind _asbp_alex (cast `/Game/ThirdPerson/Blueprints/BP_Alex` OtherActor)
        (:`then`
          (if (not (`/Game/ThirdPerson/Blueprints/BP_Alex.isShielded` _asbp_alex))
            (set `/Game/ThirdPerson/Blueprints/BP_Alex.isShielded` true _asbp_alex)))
        (:`CastFailed`
          (bind _asbp_alex_stroumph (cast `/Game/ThirdPerson/Blueprints/BP_Alex_Stroumph` OtherActor)
            (:`then`
              (if (not (`/Game/ThirdPerson/Blueprints/BP_Alex_Stroumph.isShielded` _asbp_alex_stroumph))
                (set `/Game/ThirdPerson/Blueprints/BP_Alex_Stroumph.isShielded` true _asbp_alex_stroumph)))
            (:`CastFailed`
              (bind _asbp_steve_rouge (cast `/Game/ThirdPerson/Blueprints/BP_Steve_Rouge` OtherActor))
              (if (not (`/Game/ThirdPerson/Blueprints/BP_Steve_Rouge.isShielded` _asbp_steve_rouge))
                (set `/Game/ThirdPerson/Blueprints/BP_Steve_Rouge.isShielded` true _asbp_steve_rouge))))))))
  (`self.K2_DestroyActor`))

(fn `UserConstructionScript`)