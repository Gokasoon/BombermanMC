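; Bomberman-style bomb that scales along a timeline, explodes, and destroys itself shortly after.
; Tick box-traces four directions, ignoring bombs and pickups, and applies blast effects while Boom is set, latching each direction after a non-wall hit.
; Hit characters lose their shield or die, decrementing BP_Map's player count and showing the replay menu at one or zero.
; Bricks break and randomly drop shield or BP_BonusDegat pickups.
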(event `self.ReceiveBeginPlay`
  (bind (_direction _a) (`Timeline|Timeline`)
    (:`Update`
      (`self.SetActorScale3D` (`KismetMathLibrary.Conv_DoubleToVector` _a)))
    (:`Finished`
      (`GameplayStatics.SpawnEmitterAtLocation` "/Game/StarterContent/Particles/P_Explosion.P_Explosion" (`self.K2_GetActorLocation`))
      (`GameplayStatics.PlaySound2D` "/Game/StarterContent/Audio/tnt-explosion.tnt-explosion" 1.0 1.0 0.0 null null)
      (set `self.boom` true)
      (`KismetSystemLibrary.Delay` 0.1)
      (`self.K2_DestroyActor`))))

(event `self.ReceiveTick`
  (params (DeltaSeconds :type "Float (single-precision)"))
  (bind (_returnvalue_x _returnvalue_y _returnvalue_z) (`KismetMathLibrary.BreakVector` (`self.K2_GetActorLocation`)))
  (bind _ignoredactors (`self.ignoredActors`))
  (for (_array_element _array_index) (`|MakeArray` (`KismetMathLibrary.MakeVector` (+ 300.0 _returnvalue_x) _returnvalue_y _returnvalue_z) (`KismetMathLibrary.MakeVector` (+ -300.0 _returnvalue_x) _returnvalue_y _returnvalue_z) (`KismetMathLibrary.MakeVector` _returnvalue_x (+ _returnvalue_y 300.0) _returnvalue_z) (`KismetMathLibrary.MakeVector` _returnvalue_x (+ _returnvalue_y -300.0) _returnvalue_z) :!type "Vector Structure")
    (if (not (`|GetArrayItem` (`self.endTrace`) _array_index))
      (bind _outactors (`GameplayStatics.GetAllActorsOfClass` "/Game/Actor/BP_BonusDegat.BP_BonusDegat_C"))
      (for _array_element_2 _outactors
        (`KismetArrayLibrary.Array_Add` _ignoredactors _array_element_2))
      (bind _outactors_2 (`GameplayStatics.GetAllActorsOfClass` "/Game/Actor/BP_Shield.BP_Shield_C"))
      (for _array_element_3 _outactors_2
        (`KismetArrayLibrary.Array_Add` _ignoredactors _array_element_3))
      (bind _outactors_3 (`GameplayStatics.GetAllActorsOfClass` "BP_Bomb1_C"))
      (for _array_element_4 _outactors_3
        (`KismetArrayLibrary.Array_Add` _ignoredactors _array_element_4))
      (bind _outactors_4 (`GameplayStatics.GetAllActorsOfClass` "/Game/Actor/BP_Bomb2.BP_Bomb2_C"))
      (for _array_element_5 _outactors_4
        (`KismetArrayLibrary.Array_Add` _ignoredactors _array_element_5))
      (bind _outhit (`KismetSystemLibrary.BoxTraceSingleForObjects` (`self.K2_GetActorLocation`) _array_element (20.0 20.0 20.0) (struct) (`|MakeArray` "ObjectTypeQuery1" "ObjectTypeQuery4" "ObjectTypeQuery2" "ObjectTypeQuery3" :!type "EObjectTypeQuery Enum") false _ignoredactors))
      (if (`self.boom`)
        (`/Engine/EditorBlueprintResources/StandardMacros.IsValid` (`.HitActor` (`GameplayStatics.BreakHitResult` _outhit))
          (:`Is Valid`
            (cast `/Game/Actor/BP_Wall` (`.HitActor` (`GameplayStatics.BreakHitResult` _outhit))
              (:`then`
                (`GameplayStatics.SpawnEmitterAtLocation` "/Game/StarterContent/Particles/P_Explosion.P_Explosion" (`KismetMathLibrary.VLerp` (`self.K2_GetActorLocation`) (`self.K2_GetActorLocation` (`.HitActor` (`GameplayStatics.BreakHitResult` _outhit))) 0.5)))
              (:`CastFailed`
                (cast `/Game/Actor/BP_Bomb1` (`.HitActor` (`GameplayStatics.BreakHitResult` _outhit))
                  (:`CastFailed`
                    (`KismetArrayLibrary.Array_Set` (`self.endTrace`) _array_index true)
                    (bind _returnvalue (`self.K2_GetActorLocation` (`.HitActor` (`GameplayStatics.BreakHitResult` _outhit))))
                    (`GameplayStatics.SpawnEmitterAtLocation` "/Game/StarterContent/Particles/P_Explosion.P_Explosion" _returnvalue)
                    (`GameplayStatics.SpawnEmitterAtLocation` "/Game/StarterContent/Particles/P_Explosion.P_Explosion" (`KismetMathLibrary.VLerp` _returnvalue (`self.K2_GetActorLocation`) 0.5))
                    (bind _asbp_third_person_character (cast `/Game/ThirdPerson/Blueprints/BP_ThirdPersonCharacter` (`.HitActor` (`GameplayStatics.BreakHitResult` _outhit)))
                      (:`then`
                        (if (`/Game/ThirdPerson/Blueprints/BP_ThirdPersonCharacter.isShielded` _asbp_third_person_character)
                          (set `/Game/ThirdPerson/Blueprints/BP_ThirdPersonCharacter.isShielded` false _asbp_third_person_character)
                          (else
                            (bind _outactors_5 (`GameplayStatics.GetAllActorsOfClass` "/Game/Actor/BP_Map.BP_Map_C" :!label _label))
                            (`GameplayStatics.SpawnSound2D` "/Game/StarterContent/Audio/Minecraft_Steve_OOF_Sound_Effect.Minecraft_Steve_OOF_Sound_Effect" 1.0 1.0 0.0 null)
                            (bind _output (`|GetArrayItem` _outactors_5))
                            (bind _output_get (set `/Game/Actor/BP_Map.nbPlayers` (- (`/Game/Actor/BP_Map.nbPlayers` _output) 1) _output))
                            (`self.K2_DestroyActor` (`.HitActor` (`GameplayStatics.BreakHitResult` _outhit)))
                            (if (== 1 _output_get)
                              (bind _returnvalue_2 (`|CreateWidget` "/Game/Widget/Replay_Menu.Replay_Menu_C" :!label _label_2))
                              (`UserWidget.AddToViewport` _returnvalue_2 0)
                              (bind _outactors_6 (`GameplayStatics.GetAllActorsOfClass` "/Script/Engine.PlayerController"))
                              (bind _output_2 (`|GetArrayItem` _outactors_6))
                              (`/Engine/EditorBlueprintResources/StandardMacros.IsValid` _output_2
                                (:`Is Valid`
                                  (set `PlayerController.bShowMouseCursor` true _output_2)))
                              (elif (== _output_get 0)
                                (goto _label_2))))))
                      (:`CastFailed`
                        (bind _asbp_alex (cast `/Game/ThirdPerson/Blueprints/BP_Alex` (`.HitActor` (`GameplayStatics.BreakHitResult` _outhit)))
                          (:`then`
                            (if (`/Game/ThirdPerson/Blueprints/BP_Alex.isShielded` _asbp_alex)
                              (set `/Game/ThirdPerson/Blueprints/BP_Alex.isShielded` false _asbp_alex)
                              (else
                                (goto _label))))
                          (:`CastFailed`
                            (bind _asbp_alex_stroumph (cast `/Game/ThirdPerson/Blueprints/BP_Alex_Stroumph` (`.HitActor` (`GameplayStatics.BreakHitResult` _outhit)))
                              (:`then`
                                (if (`/Game/ThirdPerson/Blueprints/BP_Alex_Stroumph.isShielded` _asbp_alex_stroumph)
                                  (set `/Game/ThirdPerson/Blueprints/BP_Alex_Stroumph.isShielded` false _asbp_alex_stroumph)
                                  (else
                                    (goto _label))))
                              (:`CastFailed`
                                (bind _asbp_steve_rouge (cast `/Game/ThirdPerson/Blueprints/BP_Steve_Rouge` (`.HitActor` (`GameplayStatics.BreakHitResult` _outhit)))
                                  (:`then`
                                    (if (`/Game/ThirdPerson/Blueprints/BP_Steve_Rouge.isShielded` _asbp_steve_rouge)
                                      (set `/Game/ThirdPerson/Blueprints/BP_Steve_Rouge.isShielded` false _asbp_steve_rouge)
                                      (else
                                        (goto _label))))
                                  (:`CastFailed`
                                    (cast `/Game/Actor/BP_Brick` (`.HitActor` (`GameplayStatics.BreakHitResult` _outhit)))
                                    (if (`KismetMathLibrary.RandomBool`)
                                      _
                                      (elif (`KismetMathLibrary.RandomBool`)
                                        (bind _returnvalue_3 (`KismetMathLibrary.Conv_VectorToTransform` (`self.K2_GetActorLocation` (`.HitActor` (`GameplayStatics.BreakHitResult` _outhit)))))
                                        (`|SpawnActorFromClass` "/Game/Actor/BP_Shield.BP_Shield_C" _returnvalue_3 "Undefined" "MultiplyWithRoot" null null)
                                        (else
                                          (`|SpawnActorFromClass` "/Game/Actor/BP_BonusDegat.BP_BonusDegat_C" _returnvalue_3 "Undefined" "MultiplyWithRoot" null null))))
                                    (`self.K2_DestroyActor` (`.HitActor` (`GameplayStatics.BreakHitResult` _outhit))))))))))))))))
          (:`Is Not Valid`
            (`GameplayStatics.SpawnEmitterAtLocation` "/Game/StarterContent/Particles/P_Explosion.P_Explosion" _array_element)
            (`GameplayStatics.SpawnEmitterAtLocation` "/Game/StarterContent/Particles/P_Explosion.P_Explosion" (`KismetMathLibrary.VLerp` (`self.K2_GetActorLocation`) _array_element 0.5))))))))

(fn `UserConstructionScript`)